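; BP_wash is the sink where the VR player washes held plates to build up a counted pile.
; A picked plate entering the box triggers splash, sound and the Washing timeline, which stops when an overlap ends.
; On completion the pawn drops the plate, which is destroyed, and a stackable plate spawns at Bp_pileSpawn, raised by the count.
; Tick polls the starter button and zeroes the count while its Switcher is 0.
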(event `self.ReceiveBeginPlay`)

(event `self.ReceiveTick`
  (params (DeltaSeconds :type "Float (single-precision)"))
  ;[1 1 1] if game startet set number of plates on pile to zero
  (bind _outactors (`GameplayStatics.GetAllActorsOfClass` "/Game/Assets/actors/BP_starter_button.BP_starter_button_C"))
  (bind _asbp_starter_button (cast `/Game/Assets/actors/BP_starter_button` (`KismetArrayLibrary.Array_Get` _outactors)))
  (switch `int` (`/Game/Assets/actors/BP_starter_button.Switcher` _asbp_starter_button)
    (:`0`
      (set `self.numberOfPlates` 0))))

(event `self.Box.OnComponentBeginOverlap`
  (params (OverlappedComponent :type "PrimitiveComponent Object Reference") (OtherActor :type "Actor Object Reference") (OtherComp :type "PrimitiveComponent Object Reference") (OtherBodyIndex :type Integer) (bFromSweep :type Boolean) (SweepResult :type "HitResult Structure (by ref)"))
  ;[1 1 1] destroy actors (plates) in hand, when moving into the sink (to wash for 1 sec), pile up (score) plates, play washing sound and show watersplash
  (bind _asbp_plate (cast `/Game/Assets/actors/BP_plate` OtherActor))
  (if (`/Game/Assets/actors/BP_plate.isPicked` _asbp_plate)
    (if (== (`GameplayStatics.GetObjectClass` OtherActor) "/Game/Assets/actors/BP_plate.BP_plate_C")
      (`self.showWaterSplash`)
      (`GameplayStatics.PlaySoundAtLocation` "/Game/Assets/audio/wave_cue.wave_cue" (`self.K2_GetActorLocation`))
      (`Timeline|washing` :!via `PlayFromStart` :!label _label
        (:`Finished`
          (bind _asmy_vr_pawn (cast `/Game/Assets/player/myVR_pawn` (`GameplayStatics.GetPlayerPawn` 0)))
          (message `/Game/Assets/actors/BPI_MyPickUpInterface.DropOff` (`/Game/Assets/player/myVR_pawn.attachedActor` _asmy_vr_pawn) (`self.GetParentComponent` OtherActor))
          (set `/Game/Assets/player/myVR_pawn.attachedActor` null _asmy_vr_pawn)
          (`self.plateCounter`)
          (`self.spawnStaple`)
          (`self.K2_DestroyActor` OtherActor))))))

(event `self.Box.OnComponentEndOverlap`
  (params (OverlappedComponent :type "PrimitiveComponent Object Reference") (OtherActor :type "Actor Object Reference") (OtherComp :type "PrimitiveComponent Object Reference") (OtherBodyIndex :type Integer))
  (goto _label :!via `Stop`))

(event `plateCounter`
  ;[1 1 1] count plates
  (set `self.numberOfPlates` (+ (`self.numberOfPlates`) 1)))

(event `spawnStaple`
  ;[1 1 1] spawn new plate on top of the pile
  (bind _outactors (`GameplayStatics.GetAllActorsOfClass` "/Game/Assets/actors/bp_pileSpawn.bp_pileSpawn_C"))
  (bind (_returnvalue_location _returnvalue_rotation _returnvalue_scale) (`KismetMathLibrary.BreakTransform` (`self.GetTransform` (`KismetArrayLibrary.Array_Get` _outactors))))
  (`|SpawnActorFromClass` "/Game/Assets/actors/bp_plate_stapable.bp_plate_stapable_C" (`KismetMathLibrary.MakeTransform` (`KismetMathLibrary.MakeVector` (.x _returnvalue_location) (.y _returnvalue_location) (+ (.z _returnvalue_location) (* (`self.numberOfPlates`) 2.0))) _returnvalue_rotation _returnvalue_scale) "AlwaysSpawn" "OverrideRootScale"))

(event `showWaterSplash`
  ;[1 1 1] toggle watersplash, while washing
  (bind _outactors (`GameplayStatics.GetAllActorsOfClass` "/Game/Assets/actors/BP_waterjet.BP_waterjet_C"))
  (bind _asbp_waterjet (cast `/Game/Assets/actors/BP_waterjet` (`KismetArrayLibrary.Array_Get` _outactors)))
  (`/Game/Assets/actors/BP_waterjet.showWater` _asbp_waterjet))

(fn `UserConstructionScript`)