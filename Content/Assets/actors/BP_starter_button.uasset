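; VR button actor that starts a timed game round, or stops an active one, when the VR pawn overlaps it.
; A Switcher state picks the action, and start, manual stop and timeout each fire their own dispatcher.
; A looping one-second timer runs the countdown and plays ticking cues near the end.
; Tick detects zero and ends the round, briefly delaying the reset to idle for BP_plate's per-tick tracking.
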(event `self.starter_button.OnComponentBeginOverlap`
  (params (OverlappedComponent :type "PrimitiveComponent Object Reference") (OtherActor :type "Actor Object Reference") (OtherComp :type "PrimitiveComponent Object Reference") (OtherBodyIndex :type Integer) (bFromSweep :type Boolean) (SweepResult :type "HitResult Structure (by ref)"))
  ;[1 1 1] depending on game state either start or stopp game actively
  (if (== (`GameplayStatics.GetObjectClass` OtherActor) "/Game/Assets/player/myVR_pawn.myVR_pawn_C")
    (switch `int` (`self.Switcher`)
      (:`0`
        (`self.StartTheGame`))
      (:`1`
        (`self.StopGameActive`)
        (`KismetSystemLibrary.K2_ClearTimer` null "Decrement")
        (set `self.Switcher` 0)))))

(event `self.ReceiveTick`
  (params (DeltaSeconds :type "Float (single-precision)"))
  ;[1 1 1] stopp game if timer has run out
  (if (== (`self.timerSeconds`) 0)
    (set `self.Switcher` 2)
    (`self.StoppTheGame`)))

(event `StartTheGame`
  ;[1 1 1] start game, play sound and start timer
  (set `self.timerSeconds` (`self.MaxTimer`))
  (`GameplayStatics.PlaySound2D` "/Game/Assets/audio/final.final")
  (`self.StartGame`)
  (set `self.Switcher` 1)
  (`KismetSystemLibrary.K2_SetTimer` null "Decrement" 1.0 true))

(event `StoppTheGame`
  ;[1 1 1] stopp game (timer basesd), stopp timer; (delay: no propper end whithout delay - tracked every tick in BP_plate)
  (`KismetSystemLibrary.K2_ClearTimer` null "Decrement")
  (`self.StopGameTimer`)
  (set `self.timerSeconds` 1)
  (`KismetSystemLibrary.Delay` 0.2)
  (set `self.Switcher` 0))

(fn `Decrement`
  (bind _timerseconds (`self.timerSeconds`))
  ;[1 1 1] Timer decrement and playing finishing "ticking" sound
  (if (>= _timerseconds 1)
    (set `self.timerSeconds` (- _timerseconds 1))
    (if (or (== (`self.timerSeconds`) 10) (== (`self.timerSeconds`) 5))
      (`GameplayStatics.PlaySound2D` "/Game/Assets/audio/ticking.ticking"))))

(fn `UserConstructionScript`)