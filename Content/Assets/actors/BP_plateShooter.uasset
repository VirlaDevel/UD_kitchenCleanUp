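; BP_plateShooter is an actor that launches BP_plate actors into the air at random intervals while the starter button is switched on.
; Tick runs into a random Delay as a repeating timer, then reads Switcher on the first BP_starter_button found in the level.
; SpawnPlate spawns a plate just above the Shooter component, applies a randomized upward impulse and a fixed angular impulse, and plays the shooting sound.
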(event `self.ReceiveBeginPlay`
  (`self.EnableInput` (`GameplayStatics.GetPlayerController` 0)))

(event `SpawnPlate`
  (bind (_returnvalue_location _returnvalue_rotation _returnvalue_scale) (`KismetMathLibrary.BreakTransform` (`SceneComponent.K2_GetComponentToWorld` (`self.shooter`))))
  ;[1 1 1] Event to spawn a plate, add some random impus (for trajectory) and play sound at location
  (bind _returnvalue (`|SpawnActorFromClass` "/Game/Assets/actors/BP_plate.BP_plate_C" (`KismetMathLibrary.MakeTransform` (`KismetMathLibrary.MakeVector` (.x _returnvalue_location) (.y _returnvalue_location) (+ (.z _returnvalue_location) 15.0)) _returnvalue_rotation _returnvalue_scale) "AlwaysSpawn" "OverrideRootScale"))
  (bind _plate (`/Game/Assets/actors/BP_plate.plate` _returnvalue))
  (`PrimitiveComponent.AddImpulse` _plate (`self.randomImpuls`) "None" false)
  (`PrimitiveComponent.AddAngularImpulse` _plate (0.0 50.0 0.0) "None" false)
  (`GameplayStatics.PlaySoundAtLocation` "/Game/Assets/audio/shootingPlate_cue.shootingPlate_cue" _returnvalue_location))

(event `self.ReceiveTick`
  (params (DeltaSeconds :type "Float (single-precision)"))
  ;[1 1 1] Spawn plates in random span of time
  (`KismetSystemLibrary.Delay` (`KismetMathLibrary.RandomFloatInRange` 2.5 6.0))
  (bind _outactors (`GameplayStatics.GetAllActorsOfClass` "/Game/Assets/actors/BP_starter_button.BP_starter_button_C"))
  (bind _asbp_starter_button (cast `/Game/Assets/actors/BP_starter_button` (`KismetArrayLibrary.Array_Get` _outactors)))
  (switch `int` (`/Game/Assets/actors/BP_starter_button.Switcher` _asbp_starter_button)
    (:`1`
      (`self.SpawnPlate`))))

(fn `randomImpuls`
  (returns (impuls :type "Vector Structure"))
  ;[1 1 1] Generates random vector for impuls
  (return (`KismetMathLibrary.MakeVector` (`KismetMathLibrary.RandomFloatInRange` 0.0 75.0) (`KismetMathLibrary.RandomFloatInRange` 15.0 75.0) (`KismetMathLibrary.RandomFloatInRange` 130.0 160.0))))

(fn `UserConstructionScript`)