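; Pickup-able plate actor that shatters into a Bp_plateBroken actor with a crash sound when hit or when the game is actively stopped.
; PickUp and DropOff interface events toggle physics and attachment, while Tick applies a constant downward force to unheld plates for a slowed fall.
; Tick also polls BP_starter_button's Switcher state to bind start and stop handlers or run the timeout, which removes plates without shattering.
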(event `StartGame`
  ;[1 1 1] depending ons game state - toggle start and stopp and destroying of actors
  ;;[0.5501 1 0.466] Start Game - desroy all existing plates
  (`self.K2_DestroyActor`))

(event `self.ReceiveTick`
  (params (DeltaSeconds :type "Float (single-precision)"))
  ;[1 1 1] physical parameter G is reduced to slow down fall (gravitiy not activatet)
  (if (not (`self.isPicked`))
    (`PrimitiveComponent.AddForce` (`self.plate`) (0.0 0.0 -110.0) "None" false))
  ;[1 1 1] depending ons game state - toggle start and stopp and destroying of actors
  (bind _outactors (`GameplayStatics.GetAllActorsOfClass` "/Game/Assets/actors/BP_starter_button.BP_starter_button_C"))
  (set `self.plateDestroyer` (`KismetArrayLibrary.Array_Get` _outactors))
  (switch `int` (`/Game/Assets/actors/BP_starter_button.Switcher` (`self.plateDestroyer`))
    (:`0`
      ;;[0.5501 1 0.466] Start Game - desroy all existing plates
      (add `/Game/Assets/actors/BP_starter_button.StartGame` (`self.plateDestroyer`) (delegate `StartGame`)))
    (:`1`
      ;;[1 0.495 0.495] Player has stopped game with button
      (add `/Game/Assets/actors/BP_starter_button.StopGameActive` (`self.plateDestroyer`) (delegate `StoppGameActive`)))
    (:`2`
      (`self.StoppGameTimer`))))

(event `StoppGameActive`
  ;[1 1 1] depending ons game state - toggle start and stopp and destroying of actors
  ;;[1 0.495 0.495] Active stopp - destroy all plates
  (`GameplayStatics.PlaySoundAtLocation` "/Game/Assets/audio/crashingPlate_cue.crashingPlate_cue" (`SceneComponent.K2_GetComponentLocation` (`self.plate`)))
  (`self.DropOff`)
  (`self.activeDestroyment`))

(event `/Game/Assets/actors/My_PickUpInterface.PickUp`
  (params (ActorToAttachTo :type "SceneComponent Object Reference"))
  ;[1 1 1] Pick up plate interface event
  (`PrimitiveComponent.SetSimulatePhysics` (`self.plate`) false)
  (`SceneComponent.K2_AttachToComponent` (`self.K2_GetRootComponent`) ActorToAttachTo "None" "KeepWorld" "KeepWorld" "KeepWorld" true)
  (set `self.isPicked` true))

(event `StoppGameTimer`
  ;[1 1 1] depending ons game state - toggle start and stopp and destroying of actors
  ;;[0.5395 0.5982 1] Time run out - destroy plates
  (`GameplayStatics.PlaySound2D` "/Game/Assets/audio/final.final")
  (`self.DropOff`)
  (`self.K2_DestroyActor`))

(event `/Game/Assets/actors/My_PickUpInterface.DropOff`
  ;[1 1 1] drop off plate interface event
  (`PrimitiveComponent.SetSimulatePhysics` (`self.plate`) true)
  (`self.K2_DetachFromActor` "KeepWorld" "KeepWorld" "KeepWorld")
  (set `self.isPicked` false))

(event `activeDestroyment`
  (bind _returnvalue (`SceneComponent.K2_GetComponentToWorld` (`self.plate`)))
  ;[1 1 1] spawn destroyed plate when hit or actively destroyed with start/stopp button
  (`|SpawnActorFromClass` "/Game/Assets/actors/bp_plateBroken.bp_plateBroken_C" _returnvalue "AdjustIfPossibleButAlwaysSpawn" "OverrideRootScale" :!label _label)
  (`GameplayStatics.PlaySoundAtLocation` "/Game/Assets/audio/crashingPlate_cue.crashingPlate_cue" (.location _returnvalue))
  (`self.K2_DestroyActor`))

(event `self.plate.OnComponentHit`
  (params (HitComponent :type "PrimitiveComponent Object Reference") (OtherActor :type "Actor Object Reference") (OtherComp :type "PrimitiveComponent Object Reference") (NormalImpulse :type "Vector Structure") (Hit :type "HitResult Structure (by ref)"))
  ;[1 1 1] spawn destroyed plate when hit or actively destroyed with start/stopp button
  (goto _label))

(fn `UserConstructionScript`)